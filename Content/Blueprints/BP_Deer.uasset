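; BP_Deer is a deer that free-roams the navmesh, alternating between walking and pausing to eat.
; From BeginPlay, it moves via AIMoveTo to a random navigable point within FreeRoamRadius, then sets IsEating for a random delay before MoveAgain repeats the loop, even after failed moves.
; IsMoving and IsChased gate new moves, though nothing here sets IsChased.
; BeginPlay also caches the default walk speed, unused in this graph.
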(event `self.ReceiveBeginPlay`
  (`|ExecutionSequence`
    (:`then_0`
      (if (not (or (`self.IsMoving?`) (`self.IsChased?`))) :!label _label
        (set `self.IsMoving?` true)
        (bind _randomlocation (`NavigationSystemV1.K2_GetRandomLocationInNavigableRadius` (`self.K2_GetActorLocation`) (`self.Free Roam Radius`) null null))
        (`|AIMoveTo` self _randomlocation null
          (:`OnSuccess`
            _)
          (:`OnFail`
            _))
        (set `self.IsMoving?` false)
        (set `self.IsEating?` true)
        (`KismetSystemLibrary.Delay` (`KismetMathLibrary.RandomFloatInRange` 5.0 10.0))
        (`self.Move Again`)
        (set `self.IsEating?` false)))
    (:`then_1`
      (set `self.Default Max Walk Speed` (`CharacterMovementComponent.MaxWalkSpeed` (`self.CharacterMovement`))))))

(event `Move Again`
  (goto _label))

(fn `UserConstructionScript`)