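; BP_GrassSpawner is an actor that sets up instanced static mesh components for grass foliage.
; On BeginPlay it creates a seed-zero random stream, builds one component per GrassTypes entry with that entry's mesh and shared start and end cull distances, and enables tick.
; The components are stored in GrassComponents; the graphs shown add no instances and contain no tick logic.
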(event `self.ReceiveBeginPlay`
  (set `self.RandomStream` (`KismetMathLibrary.MakeRandomStream` 0))
  (`self.InitializeFoliageTypes`)
  (`self.SetActorTickEnabled` true))

(fn `InitializeFoliageTypes`
  (locals (ISM :type "InstancedStaticMeshComponent Object Reference"))
  (for _array_element (`self.GrassTypes`)
    (bind _returnvalue (`AddComponent|NODE_AddInstancedStaticMeshComponent-0`))
    (bind _output_get (set `local.ISM` _returnvalue))
    (`StaticMeshComponent.SetStaticMesh` _output_get (`FoliageType_InstancedStaticMesh.Mesh` _array_element))
    (`InstancedStaticMeshComponent.SetCullDistances` (`local.ISM`) (`self.Start Distance`) (`self.End Distance`))
    (`KismetArrayLibrary.Array_Add` (`self.GrassComponents`) (`local.ISM`))))

(fn `UserConstructionScript`)