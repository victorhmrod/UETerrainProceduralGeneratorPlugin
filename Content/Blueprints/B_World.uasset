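; World actor that generates endless procedural terrain with instanced foliage around the player.
; A looping timer queues tiles by distance-based LOD, generates the closest asynchronously and draws it when its data is ready.
; Foliage waits for the mesh's physics-state creation event (collision fix), then populates from the section's vertices and frees the generator.
; A second timer updates navigation, while Tick moves listed actors to the player's XY when too far away.
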(event `OnPhysicsStateChanged`
  (params (ChangedComponent :type "PrimitiveComponent Object Reference") (StateChange :type "EComponentPhysicsStateChange Enum" :default "Created"))
  ;[0.5 1 1] Beginplay
  ;;[0.5 1 0.5] Collision Fix
  (switch `EComponentPhysicsStateChange` StateChange
    (:`Created`
      (if (> (`self.GeneratedMeshIndex`) -1)
        (`self.GenerateFoliageTile` (`self.GeneratedMeshIndex`))
        (set `self.GeneratorBusy` false)
        (set `self.GeneratedMeshIndex` -1)))))

(event `self.ReceiveBeginPlay`
  ;[0.5 1 1] Beginplay
  (if (`self.RandomizeFoliage`)
    (set `self.InitialSeed` (`KismetMathLibrary.RandomIntegerInRange` 0 1000)))
  (set `self.RandomStream` (`KismetMathLibrary.MakeRandomStream` (`self.InitialSeed`)))
  (`self.InitializeFoliageTypes`)
  (`self.Spawn Tiles Around Player`)
  (`KismetSystemLibrary.K2_SetTimer` null "Spawn Tiles Around Player" 0.3 true)
  ;;[0.5 1 0.5] Collision Fix
  (add `PrimitiveComponent.OnComponentPhysicsStateChanged` (`self.PROC_Terrain`) (delegate `OnPhysicsStateChanged`))
  (`self.NavUpdate`)
  (`KismetSystemLibrary.K2_SetTimer` null "NavUpdate" 0.3 true))

(event `Spawn Tiles Around Player`
  (bind (_x_start _x_end _y_start _y_end) (`self.GetTilesIndicesAroundPlayer`))
  ;[1 0.5 0.5] Infinite terrain generation
  (if (`self.GeneratorBusy`)
    (if (`self.TileDataReady`)
      (bind _returnvalue (`self.DrawTile`))
      (set `self.GeneratedMeshIndex` _returnvalue))
    (else
      (for _index (range _y_start (+ _y_end 1))
        (for _index_2 (range _x_start (+ _x_end 1))
          (bind _returnvalue_2 (`self.GetTileLocation` (make `IntPoint` _index_2 _index)))
          (bind _returnvalue_3 (`self.GetPlayerLocation`))
          (if (not (> (`KismetMathLibrary.Distance2D` (`KismetMathLibrary.Conv_VectorToVector2D` _returnvalue_3) _returnvalue_2) (`self.TileReplaceableDistance`)))
            (bind (_value _returnvalue_4) (`BlueprintMapLibrary.Map_Find` (`self.QueuedTiles`) (make `IntPoint` _index_2 _index)))
            (if _returnvalue_4
              (bind _returnvalue_5 (`self.GetTileLODLevel` _index_2 _index))
              (if (not (== (`.Y` (break `IntPoint` _value)) _returnvalue_5))
                (if (!= (break `IntPoint` _value) -1)
                  (`BlueprintMapLibrary.Map_Add` (`self.RemoveLODQueue`) (make `IntPoint` _index_2 _index) (make `IntPoint` (break `IntPoint` _value) (`.Y` (break `IntPoint` _value)))))
                (`BlueprintMapLibrary.Map_Add` (`self.QueuedTiles`) (make `IntPoint` _index_2 _index) (make `IntPoint` -1 _returnvalue_5) :!label _label))
              (else
                (goto _label))))))
      (bind _returnvalue_6 (`self.GetClosestQueuedTile`))
      (bind _value_2 (`BlueprintMapLibrary.Map_Find` (`self.QueuedTiles`) _returnvalue_6))
      (if (== (break `IntPoint` _value_2) -1)
        (bind (_x _y) (break `IntPoint` _returnvalue_6))
        (`self.GenerateTerrainAsync` _x _y (`.Y` (break `IntPoint` _value_2)))))))

(event `GenerateFoliageTile`
  (params (TerrainMeshSectionIndex :type Integer))
  ;[1 1 0.5] Generate Foliage Tile
  (bind _vertices (`KismetProceduralMeshLibrary.GetSectionFromProceduralMesh` (`self.PROC_Terrain`) TerrainMeshSectionIndex))
  (bind _output_get (set `self.FoliagePoints` _vertices))
  (for _array_element _output_get
    (`self.AddFoliageInstances` (+ _array_element (`self.K2_GetActorLocation`))))
  (`self.RefreshFoliage`))

(event `self.ReceiveTick`
  (params (DeltaSeconds :type "Float (single-precision)"))
  (`self.RelocateActors`))

(fn `GetPlayerPositionIndex`
  (returns (`Player X` :type Integer) (`Player Y` :type Integer))
  (bind _cellsize (`self.CellSize`))
  (bind _returnvalue (`self.GetPlayerLocation`))
  (return (`KismetMathLibrary.FTrunc` (/ (.x _returnvalue) (* _cellsize (- (`self.XVertexCount`) 1)))) (`KismetMathLibrary.FTrunc` (/ (.y _returnvalue) (* _cellsize (- (`self.YVertexCount`) 1))))))

(fn `GetTileLODLevel`
  (params (X :type Integer) (Y :type Integer))
  (returns (ReturnValue :type Integer))
  (bind _cellsize (`self.CellSize`))
  (bind _returnvalue (`self.GetPlayerLocation`))
  (return (`KismetMathLibrary.FTrunc` (`KismetMathLibrary.FMax` (`KismetMathLibrary.Distance2D` (`KismetMathLibrary.MakeVector2D` (+ X 0.5) (+ Y 0.5)) (`KismetMathLibrary.MakeVector2D` (/ (.x _returnvalue) (* _cellsize (- (`self.XVertexCount`) 1))) (/ (.y _returnvalue) (* _cellsize (- (`self.YVertexCount`) 1))))) 1.0))))

(fn `GetTilesIndicesAroundPlayer`
  (returns (`X Start` :type Integer) (`X End` :type Integer) (`Y Start` :type Integer) (`Y End` :type Integer))
  (bind (_player_x _player_y) (`self.GetPlayerPositionIndex`))
  (bind _numofsectiony (`self.NumOfSectionY`))
  (bind _numofsectionx (`self.NumOfSectionX`))
  (bind _returnvalue (- _player_y (/ _numofsectiony 2)))
  (bind _returnvalue_2 (- _player_x (/ _numofsectionx 2)))
  (return _returnvalue_2 (+ _returnvalue_2 _numofsectionx -1) _returnvalue (+ _returnvalue _numofsectiony -1)))

(fn `InitializeFoliageTypes`
  (locals (ISMComp :type "InstancedStaticMeshComponent Object Reference"))
  (for _array_element (`self.FoliageTypes`)
    (bind _returnvalue (`AddComponent|NODE_AddInstancedStaticMeshComponent-0`))
    (bind _output_get (set `local.ISMComp` _returnvalue))
    (`StaticMeshComponent.SetStaticMesh` _output_get (`FoliageType_InstancedStaticMesh.Mesh` _array_element))
    (`KismetArrayLibrary.Array_Add` (`self.FoliageComponents`) (`local.ISMComp`))
    (`InstancedStaticMeshComponent.SetCullDistances` (`local.ISMComp`) (`self.StartCullDistance`) (`self.EndCullDistance`))))

(fn `NavUpdate`
  (`WEUtilities.NavUpdate` (`self.PROC_Terrain`)))

(fn `RefreshFoliage`
  (for _array_element (`self.FoliageComponents`)
    (`InstancedStaticMeshComponent.UpdateInstanceTransform` _array_element 0 (`InstancedStaticMeshComponent.GetInstanceTransform` _array_element 0 true) true false false)))

(fn `RelocateActors`
  (for _array_element (`self.ActorsToBeRelocated`)
    (bind _returnvalue (`self.GetPlayerLocation`))
    (bind _returnvalue_2 (`self.K2_GetActorLocation` _array_element))
    (if (> (`KismetMathLibrary.Vector_Distance2D` _returnvalue _returnvalue_2) (`self.RelocateDistance`))
      (`self.K2_SetActorLocation` _array_element (`KismetMathLibrary.MakeVector` (.x _returnvalue) (.y _returnvalue) (.z _returnvalue_2)) false false))))

(fn `UserConstructionScript`)